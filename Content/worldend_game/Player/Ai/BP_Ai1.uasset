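; Sword-wielding AI enemy character with a four-montage combo, triggered through Attack, apparently from a behavior tree.
; AttackIndex selects each slash, and SwordAttackCombo continues a saved input or resets the chain.
; A looping timer sphere-traces along the blade, applying throttled damage and Niagara blood to Player-tagged actors.
; Incoming damage knocks it along the player's forward vector and feeds BPCPlayerStats, which can trigger ragdoll; health and investigation widgets face the camera.
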(event Custom|SwordAttack
  ;[0.05098 0.05098 0.05098] Combo system
  ;;[0.05098 0.05098 0.05098] Sword Attack
  (if (Variables|Default|GetisAttacking?)
    (Variables|Default|SetSave%20Attack? true)
    (else
      (Variables|Default|SetisAttacking? false)
      (switch int (Variables|Default|GetAttackIndex)
        (:0
          (CallFunction|Attack1))
        (:1
          (CallFunction|Attack2))
        (:2
          (CallFunction|Attack3))
        (:3
          (CallFunction|Attack4))))))

(event Custom|Sword%20Attack%20Combo
  ;[0.05098 0.05098 0.05098] Combo system
  ;;[0.05098 0.05098 0.05098] Combo Continue
  (if (Variables|Default|GetSave%20Attack?)
    (Variables|Default|SetSave%20Attack? false)
    (switch int (Variables|Default|GetAttackIndex)
      (:0
        (CallFunction|Attack1))
      (:1
        (CallFunction|Attack2))
      (:2
        (CallFunction|Attack3))
      (:3
        (CallFunction|Attack4)))
    (else
      (CallFunction|StopCombo))))

(event Custom|Attack3
  ;[0.05098 0.05098 0.05098] Combo system
  ;;[0.05098 0.05098 0.05098] Attack3
  (Utilities|FlowControl|DoOnce false :!label _label
    (:Completed
      (Utilities|FlowControl|Delay 0.1)
      (Animation|Montage|PlayMontage (Variables|Character|GetMesh) "/Game/worldend_game/Player/Animation_Montage/sword_and_shield_attack__2_1_Montage.sword_and_shield_attack__2_1_Montage" (Variables|Default|GetAttack%20speed)
        (:then
          (Variables|Default|SetAttackIndex 3)
          (goto _label Reset))))))

(event Custom|StopCombo
  ;[0.05098 0.05098 0.05098] Combo system
  ;;[0.05098 0.05098 0.05098] Stop Combo/Attack
  (Variables|Default|SetisAttacking? false)
  (Variables|Default|SetAttackIndex 0))

(event Custom|Ragdoll
  ;[0.05098 0.05098 0.05098] Ragdoll
  (Utilities|FlowControl|Delay 0.2)
  (Physics|SetSimulatePhysics (Variables|Character|GetMesh) true)
  (Rendering|SetVisibility (Variables|Default|GetHealthBar) false false)
  (Components|DestroyComponent (Variables|Default|GetSword)))

(event Custom|SwordAttackComboCallFromBT
  ;[0.05098 0.05098 0.05098] Combo system
  ;;[0.05098 0.05098 0.05098] Attackinput
  (if (Variables|Default|GetCanAttack)
    (CallFunction|SwordAttack)))

(event Custom|Start%20sword%20trace
  ;[0.05098 0.05098 0.05098] SwordTrace
  (bind _returnvalue (Utilities|Time|SetTimerbyEvent (delegate Custom|Sword%20trace%20loop) 0.001 true))
  (Variables|Default|SetSwordTraceLoop _returnvalue))

(event Custom|Attack4
  ;[0.05098 0.05098 0.05098] Combo system
  ;;[0.05098 0.05098 0.05098] Attack4
  (Utilities|FlowControl|DoOnce false :!label _label
    (:Completed
      (Utilities|FlowControl|Delay 0.1)
      (Animation|Montage|PlayMontage (Variables|Character|GetMesh) "/Game/worldend_game/Player/Animation_Montage/sword_and_shield_slash__4_1_Montage.sword_and_shield_slash__4_1_Montage" (Variables|Default|GetAttack%20speed)
        (:then
          (Variables|Default|SetAttackIndex 4)
          (goto _label Reset))))))

(event Custom|Sword%20trace%20loop
  ;[0.05098 0.05098 0.05098] SwordTrace
  (bind (_outhit _returnvalue) (Collision|SphereTraceByChannel (Transformation|GetWorldLocation (Variables|Default|GetSwordBottomPoint)) (Transformation|GetWorldLocation (Variables|Default|GetSwordTopPoint)) 3.0 "TraceTypeQuery1" false 0 "None" true "(R=1.000000,G=0.000000,B=0.000000,A=1.000000)" "(R=0.000000,G=1.000000,B=0.000000,A=1.000000)" 0.2))
  (if _returnvalue
    (if (Actor|ActorHasTag (.HitActor (Collision|BreakHitResult _outhit)) "Player")
      (Utilities|FlowControl|DoOnce false :!label _label
        (:Completed
          (Game|Damage|ApplyDamage (.HitActor (Collision|BreakHitResult _outhit)) (Variables|Default|GetBase%20Damage) 0 0)
          (Niagara|SpawnSystematLocation "/Game/worldend_game/Niagra/NS_Blood.NS_Blood" (.Location (Collision|BreakHitResult _outhit)) (Math|Rotator|MakeRotfromXY (.Normal (Collision|BreakHitResult _outhit)) (.Normal (Collision|BreakHitResult _outhit))) "0.200000,0.200000,0.200000")
          (Utilities|FlowControl|Delay 0.5)
          (goto _label Reset))))))

(event Custom|Attack1
  ;[0.05098 0.05098 0.05098] Combo system
  ;;[0.05098 0.05098 0.05098] Attack1
  (Utilities|FlowControl|DoOnce false :!label _label
    (:Completed
      (Utilities|FlowControl|Delay 0.1)
      (Animation|Montage|PlayMontage (Variables|Character|GetMesh) "/Game/worldend_game/Player/Animation_Montage/sword_and_shield_slash1_Montage.sword_and_shield_slash1_Montage" (Variables|Default|GetAttack%20speed)
        (:then
          (Variables|Default|SetAttackIndex 1)
          (goto _label Reset))))))

(event Custom|StopSwordTrace
  ;[0.05098 0.05098 0.05098] SwordTrace
  (Utilities|Time|ClearandInvalidateTimerbyHandle (Variables|Default|GetSwordTraceLoop)))

(event Custom|Attack2
  ;[0.05098 0.05098 0.05098] Combo system
  ;;[0.05098 0.05098 0.05098] Attack2
  (Utilities|FlowControl|DoOnce false :!label _label
    (:Completed
      (Utilities|FlowControl|Delay 0.1)
      (Animation|Montage|PlayMontage (Variables|Character|GetMesh) "/Game/worldend_game/Player/Animation_Montage/sword_and_shield_slash__3_1_Montage.sword_and_shield_slash__3_1_Montage" (Variables|Default|GetAttack%20speed)
        (:then
          (Variables|Default|SetAttackIndex 2)
          (goto _label Reset))))))

(event Custom|EnableInvestigation%20icon
  (bind _investigatewidget (Variables|Default|GetInvestigatewidget))
  (Utilities|FlowControl|FlipFlop
    (:A
      (Rendering|SetVisibility _investigatewidget true false))
    (:B
      (Rendering|SetVisibility _investigatewidget false false))))

(event EventBeginPlay
  (bind _aswb_dummy_healthbar (Utilities|Casting|CastToWB_DummyHealthbar (UserInterface|GetWidget (Variables|Default|GetHealthBar))))
  (Variables|Default|SetHealthBarUI _aswb_dummy_healthbar))

(event Collision|EventActorBeginOverlap
  (params (OtherActor :type Actor%20Object%20Reference)))

(event EventTick
  (params (DeltaSeconds :type Float%20%28single-precision%29))
  (Transformation|SetWorldRotation (Variables|Default|GetHealthBar) (Math|Rotator|FindLookatRotation (Transformation|GetWorldLocation (Variables|Default|GetHealthBar)) (Transformation|GetWorldLocation (Variables|/Script/Engine.Actor|GetRootComponent (Game|GetPlayerCameraManager 0)))) false false))

(event Game|Damage|EventAnyDamage
  (params (Damage :type Float%20%28single-precision%29) (DamageType :type Damage%20Type%20Object%20Reference) (InstigatedBy :type Controller%20Object%20Reference) (DamageCauser :type Actor%20Object%20Reference))
  (bind _asbp_playercharacter (Utilities|Casting|CastToBP_playercharacter (Game|GetPlayerCharacter 0)))
  (Character|LaunchCharacter (* (Math|Vector|GetForwardVector (Transformation|GetActorRotation _asbp_playercharacter)) 7e+02) false false)
  (bind _isplayerdead (Default|Decreasehealth (Variables|Default|GetBPC_player_stats) Damage))
  (if _isplayerdead
    (Collision|SetCollisionObjectType (Variables|Character|GetMesh) "ECC_PhysicsBody")
    (CallFunction|Ragdoll)))

(fn ConstructionScript)

(fn Attack
  (CallFunction|SwordAttackComboCallfromBT)
  (return 0.4))
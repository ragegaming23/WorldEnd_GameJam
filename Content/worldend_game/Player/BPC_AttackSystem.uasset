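; Player attack component that runs a four-step sword-and-shield melee combo, including a kick.
; Attack input calls SwordAttack, which picks a montage by AttackIndex, and starts a looping-timer sphere trace between blade sockets to damage "Enemy" actors.
; A separate kick trace damages "Damageable" actors; both spawn blood and use half-second DoOnce cooldowns.
; SwordAttackCombo, StopCombo and StopSwordTrace handle continuation and cleanup, with SaveAttack buffering input.
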(event Custom|SwordAttack
  ;[0.05098 0.05098 0.05098] Combo system
  ;;[0.05098 0.05098 0.05098] Sword Attack
  (if (Variables|Default|GetisAttacking?)
    (Variables|Default|SetSave%20Attack? true)
    (else
      (Variables|Default|SetisAttacking? false)
      (switch int (Variables|Default|GetAttackIndex)
        (:0
          (CallFunction|Attack1))
        (:1
          (CallFunction|Attack2))
        (:2
          (CallFunction|Attack3))
        (:3
          (CallFunction|Attack4))))))

(event Custom|Sword%20Attack%20Combo
  ;[0.05098 0.05098 0.05098] Combo system
  ;;[0.05098 0.05098 0.05098] Combo Continue
  (if (Variables|Default|GetSave%20Attack?)
    (Variables|Default|SetSave%20Attack? false)
    (switch int (Variables|Default|GetAttackIndex)
      (:0
        (CallFunction|Attack1))
      (:1
        (CallFunction|Attack2))
      (:2
        (CallFunction|Attack3))
      (:3
        (CallFunction|Attack4)))
    (else
      (CallFunction|StopCombo))))

(event Custom|Attack3
  ;[0.05098 0.05098 0.05098] Combo system
  ;;[0.05098 0.05098 0.05098] Attack3
  (Utilities|FlowControl|DoOnce false :!label _label
    (:Completed
      (Utilities|FlowControl|Delay 0.1)
      (Animation|Montage|PlayMontage (Variables|Default|GetCharacter%20Mesh) "/Game/worldend_game/Animation_Montage/sword_and_shield_kick1_Montage.sword_and_shield_kick1_Montage" (Variables|Default|GetPlay%20Rate)
        (:then
          (Variables|Default|SetAttackIndex 3)
          (goto _label Reset))))))

(event Custom|Weapon%20Damage
  (params (Base%20Damage :type Float%20%28single-precision%29))
  ;[0.05098 0.05098 0.05098] SwordTrace
  (Variables|Default|SetBase%20Damage Base%20Damage))

(event Custom|StopCombo
  ;[0.05098 0.05098 0.05098] Combo system
  ;;[0.05098 0.05098 0.05098] Stop Combo/Attack
  (Variables|Default|SetisAttacking? false)
  (Variables|Default|SetAttackIndex 0))

(event Custom|Start%20sword%20trace
  ;[0.05098 0.05098 0.05098] SwordTrace
  (bind _returnvalue (Utilities|Time|SetTimerbyEvent (delegate Custom|Sword%20trace%20loop) 0.001 true))
  (Variables|Default|SetSwordTraceLoop _returnvalue))

(event Custom|Attack4
  ;[0.05098 0.05098 0.05098] Combo system
  ;;[0.05098 0.05098 0.05098] Attack4
  (Utilities|FlowControl|DoOnce false :!label _label
    (:Completed
      (Utilities|FlowControl|Delay 0.1)
      (Animation|Montage|PlayMontage (Variables|Default|GetCharacter%20Mesh) "/Game/worldend_game/Animation_Montage/sword_and_shield_slash__4_1_Montage.sword_and_shield_slash__4_1_Montage" (Variables|Default|GetPlay%20Rate)
        (:then
          (Variables|Default|SetAttackIndex 4)
          (goto _label Reset))))))

(event Custom|Sword%20trace%20loop
  ;[0.05098 0.05098 0.05098] SwordTrace
  (bind (_outhit _returnvalue) (Collision|SphereTraceByChannel (Transformation|GetWorldLocation (Variables|/Game/worldend_game/Player/BP_playercharacter.BP_playercharacter_C|GetSwordBottomPoint (Variables|Default|GetCharacterBP))) (Transformation|GetWorldLocation (Variables|/Game/worldend_game/Player/BP_playercharacter.BP_playercharacter_C|GetSwordTopPoint (Variables|Default|GetCharacterBP))) 3.0 "TraceTypeQuery1" false 0 "None" true "(R=1.000000,G=0.000000,B=0.000000,A=1.000000)" "(R=0.000000,G=1.000000,B=0.000000,A=1.000000)" 0.2))
  (if _returnvalue
    (if (Actor|ActorHasTag (.HitActor (Collision|BreakHitResult _outhit)) "Enemy")
      (Utilities|FlowControl|DoOnce false :!label _label
        (:Completed
          (Game|Damage|ApplyDamage (.HitActor (Collision|BreakHitResult _outhit)) (Variables|Default|GetBase%20Damage) 0 0)
          (Niagara|SpawnSystematLocation "/Game/worldend_game/Niagra/NS_Blood.NS_Blood" (.Location (Collision|BreakHitResult _outhit)) (Math|Rotator|MakeRotfromXY (.Normal (Collision|BreakHitResult _outhit)) (.Normal (Collision|BreakHitResult _outhit))) "0.200000,0.200000,0.200000")
          (Utilities|FlowControl|Delay 0.5)
          (goto _label Reset))))))

(event Custom|Attack1
  ;[0.05098 0.05098 0.05098] Combo system
  ;;[0.05098 0.05098 0.05098] Attack1
  (Utilities|FlowControl|DoOnce false :!label _label
    (:Completed
      (Utilities|FlowControl|Delay 0.1)
      (Animation|Montage|PlayMontage (Variables|Default|GetCharacter%20Mesh) "/Game/worldend_game/Animation_Montage/sword_and_shield_slash1_Montage.sword_and_shield_slash1_Montage" (Variables|Default|GetPlay%20Rate)
        (:then
          (Variables|Default|SetAttackIndex 1)
          (goto _label Reset))))))

(event Custom|StopSwordTrace
  ;[0.05098 0.05098 0.05098] SwordTrace
  (Utilities|Time|ClearandInvalidateTimerbyHandle (Variables|Default|GetSwordTraceLoop)))

(event Custom|Attack2
  ;[0.05098 0.05098 0.05098] Combo system
  ;;[0.05098 0.05098 0.05098] Attack2
  (Utilities|FlowControl|DoOnce false :!label _label
    (:Completed
      (Utilities|FlowControl|Delay 0.1)
      (Animation|Montage|PlayMontage (Variables|Default|GetCharacter%20Mesh) "/Game/worldend_game/Animation_Montage/sword_and_shield_slash__3_1_Montage.sword_and_shield_slash__3_1_Montage" (Variables|Default|GetPlay%20Rate)
        (:then
          (Variables|Default|SetAttackIndex 2)
          (goto _label Reset))))))

(event Custom|SphereTrace
  (bind _characterbp (Variables|Default|GetCharacterBP))
  (bind _spheretrace (Variables|/Game/worldend_game/Player/BP_playercharacter.BP_playercharacter_C|GetSphereTrace _characterbp))
  (bind _returnvalue (Transformation|GetWorldLocation _spheretrace))
  ;[0.05098 0.05098 0.05098] SphereTrace(for kick)
  (bind (_outhit _returnvalue_2) (Collision|SphereTraceByChannel _returnvalue _returnvalue 25.0 "TraceTypeQuery1" false 0 "None"))
  (if _returnvalue_2
    (if (Actor|ActorHasTag (.HitActor (Collision|BreakHitResult _outhit)) "Damageable")
      (Utilities|FlowControl|DoOnce false :!label _label
        (:Completed
          (Game|Damage|ApplyDamage (.HitActor (Collision|BreakHitResult _outhit)) 1e+01 0 0)
          (Niagara|SpawnSystematLocation "/Game/worldend_game/Niagra/NS_Blood.NS_Blood" (.Location (Collision|BreakHitResult _outhit)) (Math|Rotator|MakeRotfromXY (.Normal (Collision|BreakHitResult _outhit)) (.Normal (Collision|BreakHitResult _outhit))) "0.200000,0.200000,0.200000")
          (Utilities|FlowControl|Delay 0.5)
          (goto _label Reset))))))

(event Input|EnhancedActionEvents|EnhancedInputActionIA_Attack
  (params (ActionValue :type Boolean) (ElapsedSeconds :type Float%20%28double-precision%29) (TriggeredSeconds :type Float%20%28double-precision%29) (InputAction :type Input%20Action%20Object%20Reference :default "/Game/ThirdPerson/Input/Actions/IA_Attack.IA_Attack"))
  ;[0.05098 0.05098 0.05098] Combo system
  ;;[0.05098 0.05098 0.05098] Attackinput
  (:Started
    (if (Variables|Default|GetCanAttack)
      (CallFunction|SwordAttack)
      (CallFunction|StartSwordTrace))))

(event EventBeginPlay
  (bind _asbp_playercharacter (Utilities|Casting|CastToBP_playercharacter (Components|GetOwner)))
  (Variables|Default|SetCharacterBP _asbp_playercharacter)
  (Variables|Default|SetCharacter%20Mesh (Variables|/Script/Engine.Character|GetMesh _asbp_playercharacter)))
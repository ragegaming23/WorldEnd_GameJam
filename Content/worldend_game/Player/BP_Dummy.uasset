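; BP_Dummy is a damageable dummy character that gets knocked back when hit and can collapse into a ragdoll.
; Damage launches it along the player's forward direction and passes to BPCPlayerStats, whose Decreasehealth result triggers the ragdoll.
; Ragdoll enables mesh physics after a short delay and hides the health bar.
; BeginPlay caches the health bar widget, and Tick rotates the bar to face the camera.
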(event Custom|Ragdoll
  ;[0.05098 0.05098 0.05098] Ragdoll
  (Utilities|FlowControl|Delay 0.2)
  (Physics|SetSimulatePhysics (Variables|Character|GetMesh) true)
  (Rendering|SetVisibility (Variables|Default|GetHealthBar) false false))

(event EventBeginPlay
  (bind _aswb_dummy_healthbar (Utilities|Casting|CastToWB_DummyHealthbar (UserInterface|GetWidget (Variables|Default|GetHealthBar))))
  (Variables|Default|SetHealthBarUI _aswb_dummy_healthbar))

(event Collision|EventActorBeginOverlap
  (params (OtherActor :type Actor%20Object%20Reference)))

(event EventTick
  (params (DeltaSeconds :type Float%20%28single-precision%29))
  (Transformation|SetWorldRotation (Variables|Default|GetHealthBar) (Math|Rotator|FindLookatRotation (Transformation|GetWorldLocation (Variables|Default|GetHealthBar)) (Transformation|GetWorldLocation (Variables|/Script/Engine.Actor|GetRootComponent (Game|GetPlayerCameraManager 0)))) false false))

(event Game|Damage|EventAnyDamage
  (params (Damage :type Float%20%28single-precision%29) (DamageType :type Damage%20Type%20Object%20Reference) (InstigatedBy :type Controller%20Object%20Reference) (DamageCauser :type Actor%20Object%20Reference))
  (bind _asbp_playercharacter (Utilities|Casting|CastToBP_playercharacter (Game|GetPlayerCharacter 0)))
  (Character|LaunchCharacter (* (Math|Vector|GetForwardVector (Transformation|GetActorRotation _asbp_playercharacter)) 7e+02) false false)
  (bind _isplayerdead (Default|Decreasehealth (Variables|Default|GetBPC_player_stats) Damage))
  (if _isplayerdead
    (CallFunction|Ragdoll)))

(fn ConstructionScript)
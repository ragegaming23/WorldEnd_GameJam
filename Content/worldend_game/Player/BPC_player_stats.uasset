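; Stats component for player, dummy and AI characters, tracking health, stamina, EXP and level.
; BeginPlay waits a tick, then casts the owner to set the references and flags that identify its type.
; Stat functions update values and push them straight to widgets; only Decreasehealth also supports AI and dummy health bars, the rest assume the player HUD.
; Damage and stamina drain report depletion, and full EXP triggers a level-up that resets EXP and raises its cap.
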(event EventBeginPlay
  (bind _returnvalue (Components|GetOwner))
  (Utilities|FlowControl|DelayUntilNextTick)
  (bind _asbp_playercharacter (Utilities|Casting|CastToBP_playercharacter _returnvalue)
    (:then
      (Variables|Default|SetPlayer%20Character%20BP _asbp_playercharacter)
      (Variables|Default|SetIsPlayer? true))
    (:CastFailed
      (bind _asbp_dummy (Utilities|Casting|CastToBP_Dummy _returnvalue)
        (:then
          (Variables|Default|SetDummyBP _asbp_dummy)
          (Variables|Default|SetIsPlayer? false)
          (Variables|Default|SetIsAi false))
        (:CastFailed
          (bind _asbp_ai_1 (Utilities|Casting|CastToBP_Ai1 _returnvalue))
          (Variables|Default|SetAi%20BP _asbp_ai_1)
          (Variables|Default|SetIsPlayer? false)
          (Variables|Default|SetIsAi true))))))

(event EventTick
  (params (DeltaSeconds :type Float%20%28single-precision%29)))

(fn Decreasehealth
  (params (Damage :type Float%20%28double-precision%29))
  (bind _ai_bp (Variables|Default|GetAi%20BP))
  (bind _player_character_bp (Variables|Default|GetPlayer%20Character%20BP))
  (bind _dummybp (Variables|Default|GetDummyBP))
  (bind _hudwidget (Variables|/Game/worldend_game/Player/BP_playercharacter.BP_playercharacter_C|GetHUDWidget _player_character_bp))
  (bind _healthbarui (Variables|/Game/worldend_game/Player/BP_Dummy.BP_Dummy_C|GetHealthBarUI _dummybp))
  (bind _healthbarui_2 (Variables|/Game/worldend_game/Ai/BP_Ai1.BP_Ai1_C|GetHealthBarUI _ai_bp))
  (if (not (<= (Variables|Health|GetCurrentHealth) 0.0))
    (bind _output_get (Variables|Health|SetCurrentHealth (- (Variables|Health|GetCurrentHealth) Damage)))
    (Progress|SetPercent (select (Variables|Default|GetIsPlayer?) (Variables|/Game/worldend_game/Player/UI/WB_HUD.WB_HUD_C|GetHealthBar _hudwidget) (select (Variables|Default|GetIsAi) (Variables|/Game/worldend_game/Player/UI/WB_DummyHealthbar.WB_DummyHealthbar_C|GetHealthBar _healthbarui_2) (Variables|/Game/worldend_game/Player/UI/WB_DummyHealthbar.WB_DummyHealthbar_C|GetHealthBar _healthbarui))) (/ _output_get (Variables|Health|GetMaxhealth)))
    (Rendering|Components|TextRender|SetText (select (Variables|Default|GetIsPlayer?) (Variables|/Game/worldend_game/Player/UI/WB_HUD.WB_HUD_C|Gethealthtext _hudwidget) (select (Variables|Default|GetIsAi) (Variables|/Game/worldend_game/Player/UI/WB_DummyHealthbar.WB_DummyHealthbar_C|GetHealthText _healthbarui_2) (Variables|/Game/worldend_game/Player/UI/WB_DummyHealthbar.WB_DummyHealthbar_C|GetHealthText _healthbarui))) (Utilities|Text|FormatText "{Currenthealth} / {Maxhealth}" (Variables|Health|GetCurrentHealth) (Variables|Health|GetMaxhealth)))
    (if (<= (Variables|Health|GetCurrentHealth) 0.0)
      _
      (else
        (return false))))
  (return true))

(fn IncreaseMaxHealth
  (params (Health%20Incremention :type Float%20%28double-precision%29))
  (bind _player_character_bp (Variables|Default|GetPlayer%20Character%20BP))
  (bind _hudwidget (Variables|/Game/worldend_game/Player/BP_playercharacter.BP_playercharacter_C|GetHUDWidget _player_character_bp))
  (Variables|Health|SetMaxhealth (+ (Variables|Health|GetMaxhealth) Health%20Incremention))
  (Progress|SetPercent (Variables|/Game/worldend_game/Player/UI/WB_HUD.WB_HUD_C|GetHealthBar _hudwidget) (/ (Variables|Health|GetCurrentHealth) (Variables|Health|GetMaxhealth)))
  (Rendering|Components|TextRender|SetText (Variables|/Game/worldend_game/Player/UI/WB_HUD.WB_HUD_C|Gethealthtext _hudwidget) (Utilities|Text|FormatText "{Currenthealth} / {Maxhealth}" (Variables|Health|GetCurrentHealth) (Variables|Health|GetMaxhealth))))

(fn DecreaseStamina
  (params (Stamina%20Depleted :type Float%20%28double-precision%29))
  (if (not (<= (Variables|Stamina|GetCurrentStamina) 0.0))
    (bind _output_get (Variables|Stamina|SetCurrentStamina (- (Variables|Stamina|GetCurrentStamina) Stamina%20Depleted)))
    (Progress|SetPercent (Variables|/Game/worldend_game/Player/UI/WB_HUD.WB_HUD_C|GetStaminaBar (Variables|/Game/worldend_game/Player/BP_playercharacter.BP_playercharacter_C|GetHUDWidget (Variables|Default|GetPlayer%20Character%20BP))) (/ _output_get (Variables|Stamina|GetMaxStamina)))
    (if (<= (Variables|Stamina|GetCurrentStamina) 0.0)
      _
      (else
        (return false))))
  (return true))

(fn IncreaseMaxStamina
  (params (Add%20stamina :type Float%20%28double-precision%29))
  (Variables|Stamina|SetMaxStamina (+ (Variables|Stamina|GetMaxStamina) Add%20stamina))
  (Progress|SetPercent (Variables|/Game/worldend_game/Player/UI/WB_HUD.WB_HUD_C|GetStaminaBar (Variables|/Game/worldend_game/Player/BP_playercharacter.BP_playercharacter_C|GetHUDWidget (Variables|Default|GetPlayer%20Character%20BP))) (/ (Variables|Stamina|GetCurrentStamina) (Variables|Stamina|GetMaxStamina))))

(fn IncreaseHealth
  (params (added%20health :type Float%20%28double-precision%29))
  (bind _player_character_bp (Variables|Default|GetPlayer%20Character%20BP))
  (bind _hudwidget (Variables|/Game/worldend_game/Player/BP_playercharacter.BP_playercharacter_C|GetHUDWidget _player_character_bp))
  (Variables|Health|SetCurrentHealth (+ (Variables|Health|GetCurrentHealth) added%20health))
  (if (> (Variables|Health|GetCurrentHealth) (Variables|Health|GetMaxhealth))
    (Variables|Health|SetCurrentHealth (Variables|Health|GetMaxhealth)))
  (Progress|SetPercent (Variables|/Game/worldend_game/Player/UI/WB_HUD.WB_HUD_C|GetHealthBar _hudwidget) (/ (Variables|Health|GetCurrentHealth) (Variables|Health|GetMaxhealth)))
  (Rendering|Components|TextRender|SetText (Variables|/Game/worldend_game/Player/UI/WB_HUD.WB_HUD_C|Gethealthtext _hudwidget) (Utilities|Text|FormatText "{Currenthealth} / {Maxhealth}" (Variables|Health|GetCurrentHealth) (Variables|Health|GetMaxhealth))))

(fn IncreaseStamina
  (params (Added%20Stamina :type Float%20%28double-precision%29))
  (Variables|Stamina|SetCurrentStamina (+ (Variables|Stamina|GetCurrentStamina) Added%20Stamina))
  (if (> (Variables|Stamina|GetCurrentStamina) (Variables|Stamina|GetMaxStamina))
    (bind _output_get (Variables|Stamina|SetCurrentStamina (Variables|Stamina|GetMaxStamina))))
  (Progress|SetPercent (Variables|/Game/worldend_game/Player/UI/WB_HUD.WB_HUD_C|GetStaminaBar (Variables|/Game/worldend_game/Player/BP_playercharacter.BP_playercharacter_C|GetHUDWidget (Variables|Default|GetPlayer%20Character%20BP))) (/ _output_get (Variables|Stamina|GetMaxStamina))))

(fn IncreaseExp
  (params (Added%20Exp :type Float%20%28double-precision%29))
  (Variables|XP|SetEXP (+ (Variables|XP|GetEXP) Added%20Exp))
  (if (>= (Variables|XP|GetEXP) (Variables|XP|GetMax_EXP))
    (LevelAndExp|IncreaseLevel 1))
  (Progress|SetPercent (Variables|/Game/worldend_game/Player/UI/WB_HUD.WB_HUD_C|GetExpBar (Variables|/Game/worldend_game/Player/BP_playercharacter.BP_playercharacter_C|GetHUDWidget (Variables|Default|GetPlayer%20Character%20BP))) (/ (Variables|XP|GetEXP) (Variables|XP|GetMax_EXP)))
  (Rendering|Components|TextRender|SetText (Variables|/Game/worldend_game/Player/UI/WB_HUD.WB_HUD_C|GetExpText (Variables|/Game/worldend_game/Player/BP_playercharacter.BP_playercharacter_C|GetHUDWidget (Variables|Default|GetPlayer%20Character%20BP))) (Utilities|Text|FormatText "{CurrentExp} / {MaxExp}" (Variables|XP|GetEXP) (Variables|XP|GetMax_EXP))))

(fn IncreaseLevel
  (params (Added%20Level :type Integer))
  (Variables|XP|SetLevel (+ (Variables|XP|GetLevel) Added%20Level))
  (Variables|XP|SetMax_EXP (+ (Variables|XP|GetMax_EXP) 1.5e+02))
  (Variables|XP|SetEXP 0.0)
  (Rendering|Components|TextRender|SetText (Variables|/Game/worldend_game/Player/UI/WB_HUD.WB_HUD_C|GetLevelText (Variables|/Game/worldend_game/Player/BP_playercharacter.BP_playercharacter_C|GetHUDWidget (Variables|Default|GetPlayer%20Character%20BP))) (Utilities|Text|ToText(Integer) (Variables|XP|GetLevel))))
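; Anim notify state that opens and closes the sword hit-trace window during attack animations.
; On begin, it starts the sword trace on the mesh owner; on end, it stops it.
; For BP_playercharacter the call goes to its BPCAttackSystm component, while BP_Ai1 owners receive it directly on the character.
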(fn ReceivedNotifyBegin
  (params (MeshComp :type Skeletal%20Mesh%20Component%20Object%20Reference) (Animation :type Anim%20Sequence%20Base%20Object%20Reference) (TotalDuration :type Float%20%28single-precision%29) (EventReference :type Anim%20Notify%20Event%20Reference%20Structure%20%28by%20ref%29))
  (bind _returnvalue (Components|GetOwner MeshComp))
  (bind _asbp_playercharacter (Utilities|Casting|CastToBP_playercharacter _returnvalue)
    (:then
      (Default|StartSwordTrace (Variables|/Game/worldend_game/Player/BP_playercharacter.BP_playercharacter_C|GetBPC_AttackSystm _asbp_playercharacter)))
    (:CastFailed
      (bind _asbp_ai_1 (Utilities|Casting|CastToBP_Ai1 _returnvalue))
      (Default|StartSwordTrace _asbp_ai_1)))
  (return false))

(fn ReceivedNotifyEnd
  (params (MeshComp :type Skeletal%20Mesh%20Component%20Object%20Reference) (Animation :type Anim%20Sequence%20Base%20Object%20Reference) (EventReference :type Anim%20Notify%20Event%20Reference%20Structure%20%28by%20ref%29))
  (bind _returnvalue (Components|GetOwner MeshComp))
  (bind _asbp_playercharacter (Utilities|Casting|CastToBP_playercharacter _returnvalue)
    (:then
      (Default|StopSwordTrace (Variables|/Game/worldend_game/Player/BP_playercharacter.BP_playercharacter_C|GetBPC_AttackSystm _asbp_playercharacter)))
    (:CastFailed
      (bind _asbp_ai_1 (Utilities|Casting|CastToBP_Ai1 _returnvalue))
      (Default|StopSwordTrace _asbp_ai_1)))
  (return false))
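; Player equipment component that handles weapon pickup and the equipment menu.
; On interact, a camera-forward sphere trace finds a BP_Weapon, appends its ItemData to WeaponSlots and destroys the actor.
; The menu input toggles WB_equipment, switching cursor and input mode and blocking attacks (via BPCAttackSystm) and movement while open.
; The R key prints the stored row names.
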(event Input|EnhancedActionEvents|EnhancedInputActionIA_interact
  (params (ActionValue :type Boolean) (ElapsedSeconds :type Float%20%28double-precision%29) (TriggeredSeconds :type Float%20%28double-precision%29) (InputAction :type Input%20Action%20Object%20Reference :default "/Game/ThirdPerson/Input/Actions/IA_interact.IA_interact"))
  (bind _follow_camera (Variables|Default|GetFollow%20Camera))
  (bind _returnvalue (Transformation|GetWorldLocation _follow_camera))
  ;[0.05098 0.05098 0.05098] PickUpTrace
  (:Started
    (bind (_outhit _returnvalue_2) (Collision|SphereTraceForObjects _returnvalue (+ _returnvalue (* (Math|Vector|GetForwardVector (Transformation|GetWorldRotation _follow_camera)) 1e+03)) 15.0 (Utilities|Array|MakeArray "ObjectTypeQuery2") false 0 "ForDuration"))
    (if _returnvalue_2
      (bind _asbp_weapon (Utilities|Casting|CastToBP_Weapon (.HitActor (Collision|BreakHitResult _outhit))))
      (CallFunction|AddWeapon (Variables|/Game/worldend_game/equipmentsystem/BP_Weapon.BP_Weapon_C|GetItemData _asbp_weapon))
      (Actor|DestroyActor _asbp_weapon)
      (Development|PrintString "PickUp"))))

(event Input|EnhancedActionEvents|EnhancedInputActionIA_EquipMenu
  (params (ActionValue :type Boolean) (ElapsedSeconds :type Float%20%28double-precision%29) (TriggeredSeconds :type Float%20%28double-precision%29) (InputAction :type Input%20Action%20Object%20Reference :default "/Game/ThirdPerson/Input/Actions/IA_EquipMenu.IA_EquipMenu"))
  (bind _returnvalue (Game|GetPlayerController 0))
  (bind _bpc_attack_systm (Variables|Default|GetBPC%20Attack%20Systm))
  (:Started
    ;[0.05098 0.05098 0.05098] Equipment menu panel
    (if (not (Variables|Default|GetIsPanelOpen?))
      (Variables|/Game/worldend_game/Player/BPC_AttackSystem.BPC_AttackSystem_C|SetCanAttack _bpc_attack_systm false)
      (Variables|Default|SetIsPanelOpen? true)
      (bind _returnvalue_2 (UserInterface|CreateWidget "/Game/worldend_game/equipmentsystem/UI/WB_equipment.WB_equipment_C"))
      (bind _output_get (Variables|Default|SetEquipmentWidget _returnvalue_2))
      (UserInterface|Viewport|AddtoViewport _output_get 0)
      (Variables|/Script/Engine.PlayerController|SetbShowMouseCursor _returnvalue true)
      (Input|SetInputModeGameandUI _returnvalue (Variables|Default|GetEquipmentWidget) "DoNotLock" true false)
      (bind _asbp_playercharacter (Utilities|Casting|CastToBP_playercharacter (Components|GetOwner)))
      (Pawn|Components|CharacterMovement|SetMovementMode (Variables|/Script/Engine.Character|GetCharacterMovement _asbp_playercharacter) "MOVE_None" 0)
      (else
        (Variables|/Game/worldend_game/Player/BPC_AttackSystem.BPC_AttackSystem_C|SetCanAttack _bpc_attack_systm true)
        (Variables|Default|SetIsPanelOpen? false)
        (bind _equipmentwidget (Variables|Default|GetEquipmentWidget)
          (:then
            (Widget|RemovefromParent _equipmentwidget)
            (Variables|Default|SetEquipmentWidget 0)
            (Variables|/Script/Engine.PlayerController|SetbShowMouseCursor _returnvalue false)
            (Input|SetInputModeGameOnly _returnvalue false)
            (bind _asbp_playercharacter_2 (Utilities|Casting|CastToBP_playercharacter (Components|GetOwner)))
            (Pawn|Components|CharacterMovement|SetMovementMode (Variables|/Script/Engine.Character|GetCharacterMovement _asbp_playercharacter_2) "MOVE_Walking" 0))
          (:else))))))

(event EventBeginPlay
  (bind _asbp_playercharacter (Utilities|Casting|CastToBP_playercharacter (Components|GetOwner)))
  (Variables|Default|SetFollow%20Camera (Variables|/Game/worldend_game/Player/BP_playercharacter.BP_playercharacter_C|GetFollowCamera _asbp_playercharacter))
  (Variables|Default|SetBPC%20Attack%20Systm (Variables|/Game/worldend_game/Player/BP_playercharacter.BP_playercharacter_C|GetBPC_AttackSystm _asbp_playercharacter)))

(event Input|KeyboardEvents|R
  (params (Key :type Key%20Structure :default "None"))
  ;[0.05098 0.05098 0.05098] PickUpTrace
  (:Pressed
    (for _array_element (Variables|Default|GetWeaponSlots)
      (Development|PrintString (Utilities|String|ToString(Name) (.rowname (.item _array_element)))))))

(fn AddWeapon
  (params (NewItem :type S%20Slots%20Structure%20%28by%20ref%29))
  (Utilities|Array|Add (Variables|Default|GetWeaponSlots) NewItem))